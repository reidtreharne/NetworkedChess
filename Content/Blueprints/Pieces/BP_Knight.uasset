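; BP_Knight is a chess-style knight piece that supplies the tiles it can move to from a given tile.
; GetAvailableMoves calls GetTilesFromMove once for each of the eight L-shaped forward/right offsets, appends the results into one output array and returns it.
; The event graph and construction script add no logic of their own.
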(event EventBeginPlay
  (|CallParentFunction) ; This node is disabled and will not be called.\nDrag off pins to build functionality.
)

(event Collision|EventActorBeginOverlap
  (params (OtherActor :type Actor%20Object%20Reference))
  (|CallParentFunction OtherActor) ; This node is disabled and will not be called.\nDrag off pins to build functionality.
)

(event EventTick
  (params (DeltaSeconds :type Float%20%28single-precision%29))
  (|CallParentFunction DeltaSeconds) ; This node is disabled and will not be called.\nDrag off pins to build functionality.
)

(fn ConstructionScript
  (|CallParentFunction))

(fn GetAvailableMoves
  (params (StartTile :type Tile%20Structure))
  (Utilities|FlowControl|Sequence
    (:then_0
      (Utilities|FlowControl|Sequence
        (:then_0
          (bind _tiles (CallFunction|GetTilesfromMove StartTile 2 1 "NewEnumerator0"))
          (Utilities|Array|AppendArray (LocalVariables|GetOutput) _tiles)
          (bind _tiles_2 (CallFunction|GetTilesfromMove StartTile 2 -1 "NewEnumerator0"))
          (Utilities|Array|AppendArray (LocalVariables|GetOutput) _tiles_2))
        (:then_1
          (bind _tiles_3 (CallFunction|GetTilesfromMove StartTile -2 1 "NewEnumerator0"))
          (Utilities|Array|AppendArray (LocalVariables|GetOutput) _tiles_3)
          (bind _tiles_4 (CallFunction|GetTilesfromMove StartTile -2 -1 "NewEnumerator0"))
          (Utilities|Array|AppendArray (LocalVariables|GetOutput) _tiles_4))
        (:then_2
          (bind _tiles_5 (CallFunction|GetTilesfromMove StartTile 1 2 "NewEnumerator0"))
          (Utilities|Array|AppendArray (LocalVariables|GetOutput) _tiles_5)
          (bind _tiles_6 (CallFunction|GetTilesfromMove StartTile -1 2 "NewEnumerator0"))
          (Utilities|Array|AppendArray (LocalVariables|GetOutput) _tiles_6))
        (:then_3
          (bind _tiles_7 (CallFunction|GetTilesfromMove StartTile 1 -2 "NewEnumerator0"))
          (Utilities|Array|AppendArray (LocalVariables|GetOutput) _tiles_7)
          (bind _tiles_8 (CallFunction|GetTilesfromMove StartTile -1 -2 "NewEnumerator0"))
          (Utilities|Array|AppendArray (LocalVariables|GetOutput) _tiles_8))))
    (:then_1
      (return (LocalVariables|GetOutput)))))