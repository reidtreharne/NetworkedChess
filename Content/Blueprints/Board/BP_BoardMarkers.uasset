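; BP_BoardMarkers draws highlight markers for the hovered and selected tiles on the game board.
; The construction script gives two instanced mesh components their own dynamic instances of M_TileHighlight, yellow for hover and blue for selection.
; Set functions clear their component and add one flattened world-space instance at the given location, so each marker shows one tile at a time.
; Clear functions remove markers individually or together.
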(fn ConstructionScript
  (Utilities|FlowControl|Sequence
    (:then_0
      (bind _returnvalue (Rendering|Material|CreateDynamicMaterialInstance "/Game/Blueprints/Materials/M_TileHighlight.M_TileHighlight" "None" :!class /Script/Engine.KismetMaterialLibrary))
      (Rendering|Material|SetVectorParameterValue _returnvalue "Color" "(R=1.000000,G=0.908542,B=0.000000,A=1.000000)" :!class /Script/Engine.MaterialInstanceDynamic)
      (Rendering|Material|SetMaterial (Variables|Default|GetHoveredTile) 0 _returnvalue))
    (:then_1
      (bind _returnvalue_2 (Rendering|Material|CreateDynamicMaterialInstance "/Game/Blueprints/Materials/M_TileHighlight.M_TileHighlight" "None" :!class /Script/Engine.KismetMaterialLibrary))
      (Rendering|Material|SetVectorParameterValue _returnvalue_2 "Color" "(R=0.000000,G=0.294236,B=1.000000,A=1.000000)" :!class /Script/Engine.MaterialInstanceDynamic)
      (Rendering|Material|SetMaterial (Variables|Default|GetSelectedTile) 0 _returnvalue_2))))

(fn SetHoveredTile
  (params (Location :type Vector))
  (CallFunction|ClearHoveredTile)
  (Class|InstancedStaticMeshComponent|AddInstanceWorldSpace (Variables|Default|GetHoveredTile) (Math|Transform|MakeTransform Location "0, 0, 0" "0.650000,0.650000,0.090000")))

(fn ClearHoveredTile
  (Components|InstancedStaticMesh|ClearInstances (Variables|Default|GetHoveredTile)))

(fn SetSelectedTile
  (params (Location :type Vector))
  (CallFunction|ClearSelectedTile)
  (Class|InstancedStaticMeshComponent|AddInstanceWorldSpace (Variables|Default|GetSelectedTile) (Math|Transform|MakeTransform Location "0, 0, 0" "0.650000,0.650000,0.100000")))

(fn ClearSelectedTile
  (Components|InstancedStaticMesh|ClearInstances (Variables|Default|GetSelectedTile)))

(fn ClearAll
  (CallFunction|ClearHoveredTile)
  (CallFunction|ClearSelectedTile))